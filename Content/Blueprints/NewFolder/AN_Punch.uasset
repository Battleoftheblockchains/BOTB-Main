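; AN_Punch is an animation notify, apparently for PaperZD, that applies punch hit detection and damage.
; On notify, it box-overlaps pawns at the render component's PunchAttack socket, excluding the owning actor, and applies fixed damage to each hit.
; It draws a debug box, even without a valid owning instance, and prints debug messages.
; PunchStrength only triggers a debug print, without affecting damage.
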(event `self.OnReceiveNotify`
  (params (OwningInstance :type "PaperZDAnimInstance Object Reference"))
  (bind _extent (`self.Extent`))
  (bind (_extent_x _extent_y _extent_z) (`KismetMathLibrary.BreakVector` (`self.Extent`)))
  (bind _returnvalue (`SceneComponent.GetSocketLocation` (`self.SequenceRenderComponent`) "PunchAttack"))
  (`/Engine/EditorBlueprintResources/StandardMacros.IsValid` OwningInstance
    (:`Is Valid`
      (bind _outactors (`KismetSystemLibrary.BoxOverlapActors` _returnvalue _extent (`|MakeArray` "ObjectTypeQuery3" :!type "EObjectTypeQuery Enum") null (`|MakeArray` (`PaperZDAnimInstance.GetOwningActor` OwningInstance))))
      (for _array_element _outactors
        (`KismetSystemLibrary.PrintString` (`KismetSystemLibrary.GetDisplayName` _array_element))
        (`GameplayStatics.ApplyDamage` _array_element 10.0))
      (`KismetSystemLibrary.PrintString` "NO MORE ACTORS FOUND")
      (`KismetSystemLibrary.DrawDebugBox` _returnvalue (`KismetMathLibrary.MakeVector` _extent_x 0.0 _extent_z) (struct :`R` 1.0 :`G` 0.577724 :`A` 1.0) (struct) 1.0)
      (if (== (`self.PunchStrength`) 1)
        (`KismetSystemLibrary.PrintString` "Medium Punch")))
    (:`Is Not Valid`
      (`KismetSystemLibrary.DrawDebugBox` _returnvalue _extent (struct :`R` 1.0 :`G` 0.476841 :`A` 1.0) (struct) 1.0))))