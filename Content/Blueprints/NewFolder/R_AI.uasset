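; R_AI is a side-view fighter character that, despite the AI name, is driven by input events for movement, jumping and three punch strengths.
; Movement runs along the X axis, and every Tick snaps control yaw to face the direction of travel.
; Punches, jumps and walking off ledges trigger animation node jumps on the AnimationComponent's AnimInstance.
; Incoming damage is only printed on screen, with no health handling.
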(event `self.ReceiveAnyDamage`
  (params (Damage :type "Float (single-precision)") (DamageType :type "DamageType Object Reference") (InstigatedBy :type "Controller Object Reference") (DamageCauser :type "Actor Object Reference"))
  (`KismetSystemLibrary.PrintString` (`KismetStringLibrary.Concat_StrStr` "Taken Damage:" (`KismetStringLibrary.Conv_DoubleToString` Damage)) true true (struct :`R` 1.0 :`G` 0.042102 :`A` 1.0) 4.0))

(event `self.ReceiveTick`
  (params (DeltaSeconds :type "Float (single-precision)"))
  (`self.Update Control Rotation`))

(event `InputAxis|MoveRight`
  (params (AxisValue :type "Float (single-precision)"))
  (`self.AddMovementInput` (`KismetMathLibrary.MakeVector` AxisValue)))

(event `Update Control Rotation`
  (`/Engine/EditorBlueprintResources/StandardMacros.CompareFloat` (.x (`MovementComponent.Velocity` (`self.CharacterMovement`)))
    (:`>`
      (`Controller.SetControlRotation` (`self.GetController`) (`KismetMathLibrary.MakeRotator` 0.0)))
    (:`<`
      (`Controller.SetControlRotation` (`self.GetController`) (`KismetMathLibrary.MakeRotator` 0.0 0.0 180.0)))))

(event `InputAction|Jump`
  (params (Key :type "Key Structure"))
  (:`Pressed`
    (`self.Jump`)))

(event `self.OnWalkingOffLedge`
  (params (PreviousFloorImpactNormal :type "Vector Structure (by ref)") (PreviousFloorContactNormal :type "Vector Structure (by ref)") (PreviousLocation :type "Vector Structure (by ref)") (TimeDelta :type "Float (single-precision)"))
  (`PaperZDAnimInstance.JumpToNode` (`PaperZDAnimationComponent.AnimInstance` (`self.AnimationComponent`)) "Airborne" "None" :!label _label))

(event `self.OnJumped`
  (goto _label))

(event `InputAction|Light Punch`
  (params (Key :type "Key Structure"))
  (:`Pressed`
    (`PaperZDAnimInstance.JumpToNode` (`PaperZDAnimationComponent.AnimInstance` (`self.AnimationComponent`)) "LP" "None")))

(event `InputAction|Medium Punch`
  (params (Key :type "Key Structure"))
  (:`Pressed`
    (`PaperZDAnimInstance.JumpToNode` (`PaperZDAnimationComponent.AnimInstance` (`self.AnimationComponent`)) "MP" "None")))

(event `InputAction|HeavyPUnch`
  (params (Key :type "Key Structure"))
  (:`Pressed`
    (`PaperZDAnimInstance.JumpToNode` (`PaperZDAnimationComponent.AnimInstance` (`self.AnimationComponent`)) "HP" "None")))

(fn `UserConstructionScript`)